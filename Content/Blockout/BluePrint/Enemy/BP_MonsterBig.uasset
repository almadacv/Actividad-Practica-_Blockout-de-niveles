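; BP_MonsterBig is an enemy monster that chases the player character.
; Every tick it casts player 0's character to BP_ThirdPersonCharacter and issues an AIMoveTo toward it.
; BeginPlay caches the first two BP_Door actors found in the level as door references.
; The MOnsterDestroy event only destroys the monster, as the call to DestroyDoordos on the second door is unconnected and never runs.
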(event Custom|MOnsterDestroy
  (Actor|DestroyActor))

(event EventBeginPlay
  (bind _outactors (Actor|GetAllActorsOfClass "/Game/Blockout/BluePrint/Misc/BP_Door.BP_Door_C"))
  (Variables|Default|SetDoor%20ref (Utilities|Array|Get(acopy) _outactors))
  (Variables|Default|SetDoor_Ref2 (Utilities|Array|Get(acopy) _outactors 1)))

(event Collision|EventActorBeginOverlap
  (params (OtherActor :type Actor%20Object%20Reference)))

(event EventTick
  (params (DeltaSeconds :type Float%20%28single-precision%29))
  (bind _asbp_third_person_character (Utilities|Casting|CastToBP_ThirdPersonCharacter (Game|GetPlayerCharacter 0)))
  (AI|AIMoveTo self "0, 0, 0" _asbp_third_person_character 1e+01 false))

(fn ConstructionScript)