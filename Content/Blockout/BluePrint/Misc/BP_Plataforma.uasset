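; BP_Plataforma is a moving platform that travels to an end position while the third-person character is inside its trigger box.
; On overlap, a timeline plays at a rate derived from Duration, lerping Mainplata's relative location from its starting point to Endlocal.
; Leaving the box reverses the timeline from its current position.
; Setup code applying mesh, scale and rotation to the platform and an end-position mesh is disconnected and never runs.
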(event OnComponentBeginOverlap(Box)
  (params (OverlappedComponent :type Primitive%20Component%20Object%20Reference) (OtherActor :type Actor%20Object%20Reference) (OtherComp :type Primitive%20Component%20Object%20Reference) (OtherBodyIndex :type Integer) (bFromSweep :type Boolean) (SweepResult :type Hit%20Result%20Structure%20%28by%20ref%29))
  (Utilities|Casting|CastToBP_ThirdPersonCharacter OtherActor)
  (Components|Timeline|SetPlayRate (Variables|Default|Getmoveplata) (/ 1.0 (Variables|Default|GetDuration)))
  (bind _moveplatagormatrack (Timeline|moveplata Play)
    (:Update
      (Transformation|SetRelativeLocation (Variables|Default|Getmainplata) (Math|Vector|Lerp(Vector) (Variables|Default|GetStartLocal) (Variables|Default|GetEndlocal) _moveplatagormatrack) false false))))

(event OnComponentEndOverlap(Box)
  (params (OverlappedComponent :type Primitive%20Component%20Object%20Reference) (OtherActor :type Actor%20Object%20Reference) (OtherComp :type Primitive%20Component%20Object%20Reference) (OtherBodyIndex :type Integer))
  (Utilities|Casting|CastToBP_ThirdPersonCharacter OtherActor)
  (Components|Timeline|SetPlayRate (Variables|Default|Getmoveplata) (/ 1.0 (Variables|Default|GetDuration)))
  (bind _moveplatagormatrack (Timeline|moveplata Reverse)
    (:Update
      (Transformation|SetRelativeLocation (Variables|Default|Getmainplata) (Math|Vector|Lerp(Vector) (Variables|Default|GetStartLocal) (Variables|Default|GetEndlocal) _moveplatagormatrack) false false))))

(event EventBeginPlay
  (Variables|Default|SetStartLocal (Variables|/Script/Engine.SceneComponent|GetRelativeLocation (Variables|Default|Getmainplata))))

(fn ConstructionScript)