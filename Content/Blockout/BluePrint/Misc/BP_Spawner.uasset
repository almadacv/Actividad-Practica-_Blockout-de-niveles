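; Spawner actor that keeps BP_Ghost minions topped up at random navmesh points around its box component.
; The SpawnMininions event enables spawning, after which Tick spawns a ghost whenever the world's ghost count is at or below NEnemies and MonsterDead is false.
; GetSpawnTransform picks a navigable location within a radius from the box's XY extent.
; BeginPlay caches the first BP_MonsterBig, but the monster destroy and spawn logic is unconnected.
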(event Custom|SpawnMininions
  (Development|PrintString "Hello")
  (Variables|Default|SetexeFirst true)
  (bind _outactors (Actor|GetAllActorsOfClass "/Game/Blockout/BluePrint/Enemy/BP_Ghost.BP_Ghost_C"))
  (if (not (Variables|Default|GetMonsterDead))
    (if (<= (Utilities|Array|Length _outactors) (Variables|Default|GetnEnemies))
      (bind _transform (Utilities|GetSpawnTransform (Variables|Default|GetScale))
        (:out
          (Game|SpawnActorfromClass "/Game/Blockout/BluePrint/Enemy/BP_Ghost.BP_Ghost_C" _transform "AdjustIfPossibleButAlwaysSpawn" 0 0))))))

(event EventBeginPlay
  (bind _outactors (Actor|GetAllActorsOfClass "/Game/Blockout/BluePrint/Enemy/BP_MonsterBig.BP_MonsterBig_C"))
  (Variables|Default|SetMonster_ref (Utilities|Array|Get(acopy) _outactors)))

(event Collision|EventActorBeginOverlap
  (params (OtherActor :type Actor%20Object%20Reference)))

(event EventTick
  (params (DeltaSeconds :type Float%20%28single-precision%29))
  (Utilities|FlowControl|Sequence
    (:then_0
      (if (Variables|Default|GetexeFirst)
        (bind _outactors (Actor|GetAllActorsOfClass "/Game/Blockout/BluePrint/Enemy/BP_Ghost.BP_Ghost_C"))
        (if (not (Variables|Default|GetMonsterDead))
          (if (<= (Utilities|Array|Length _outactors) (Variables|Default|GetnEnemies))
            (bind _transform (Utilities|GetSpawnTransform (Variables|Default|GetScale))
              (:out
                (Game|SpawnActorfromClass "/Game/Blockout/BluePrint/Enemy/BP_Ghost.BP_Ghost_C" _transform "AdjustIfPossibleButAlwaysSpawn" 0 0)))))))))

(fn ConstructionScript)